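; Stats component that manages RPG attributes and their nested stats, each split into Default, Bonus and Total values, with debug keys for testing.
; Attribute changes scale inherited stats, and modify functions refresh the UI.
; Conditional checks cap Health and Mana, trigger death, and convert full Exp into level-ups that award attribute points.
; Attributes load through the GameInstance on BeginPlay and save through it on demand.
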(event Custom|Load%20Attributes
  (bind _saved_attributes (Class|BISystem|LoadAttributes(Message) (Game|GetGameInstance)))
  (Variables|Default|SetAttributes _saved_attributes)
  (Default|CallUpdateUI))

(event Custom|Save%20Attributes
  (Class|BISystem|SaveAttributes(Message) (Game|GetGameInstance) (Variables|Default|GetAttributes)))

(event Custom|Check%20Exp
  (bind _return_value (Stats|Getters|GetStatValue "NewEnumerator2" "NewEnumerator9"))
  (bind _return_value_2 (Stats|Getters|GetStatValue "NewEnumerator2" "NewEnumerator8"))
  (if (>= _return_value _return_value_2)
    (Stats|Setters|SetStat "NewEnumerator0" "NewEnumerator9" (- _return_value _return_value_2))
    (Attributes|Function|ModifyAttribute "NewEnumerator0" "NewEnumerator0" "NewEnumerator3" 1.0)))

(event Custom|Check%20Health
  (bind _return_value (Stats|Getters|GetStatValue "NewEnumerator2" "NewEnumerator2"))
  (if (<= _return_value 0.0)
    (Default|CallOnDeath)
    (elif (> _return_value (Stats|Getters|GetStatValue "NewEnumerator2" "NewEnumerator1"))
      (Stats|Setters|SetStat "NewEnumerator0" "NewEnumerator2" (Stats|Getters|GetStatValue "NewEnumerator0" "NewEnumerator1"))
      (Stats|Setters|SetStat "NewEnumerator1" "NewEnumerator2" (Stats|Getters|GetStatValue "NewEnumerator1" "NewEnumerator1")))))

(event Custom|Check%20Mana
  (if (> (Stats|Getters|GetStatValue "NewEnumerator2" "NewEnumerator6") (Stats|Getters|GetStatValue "NewEnumerator2" "NewEnumerator5"))
    (Stats|Setters|SetStat "NewEnumerator0" "NewEnumerator6" (Stats|Getters|GetStatValue "NewEnumerator0" "NewEnumerator5"))
    (Stats|Setters|SetStat "NewEnumerator1" "NewEnumerator6" (Stats|Getters|GetStatValue "NewEnumerator1" "NewEnumerator5"))))

(event EventBeginPlay
  (CallFunction|LoadAttributes))

(event Input|KeyboardEvents|DebugKey2
  (params (Key :type Key%20Structure :default "None") (ActionValue :type Input%20Action%20Value%20Structure))
  (:Pressed
    (Stats|Functions|ModifyStat "NewEnumerator1" "NewEnumerator2" "NewEnumerator6" 1e+01)
    (Development|PrintString "Subtract Stat")))

(event Input|KeyboardEvents|DebugKeyR
  (params (Key :type Key%20Structure :default "None") (ActionValue :type Input%20Action%20Value%20Structure))
  (:Pressed
    (SaveGame|DeleteGameinSlot "Attributes")))

(event Input|KeyboardEvents|DebugKey3
  (params (Key :type Key%20Structure :default "None") (ActionValue :type Input%20Action%20Value%20Structure))
  (:Pressed
    (Attributes|Function|ModifyAttribute "NewEnumerator0" "NewEnumerator0" "NewEnumerator3" 1.0)
    (Development|PrintString "Add Attribute")))

(event Input|KeyboardEvents|DebugKey4
  (params (Key :type Key%20Structure :default "None") (ActionValue :type Input%20Action%20Value%20Structure))
  (:Pressed
    (Attributes|Function|ModifyAttribute "NewEnumerator1" "NewEnumerator0" "NewEnumerator7" 1.0)
    (Development|PrintString "Subtract Attribute")))

(event Input|KeyboardEvents|DebugKeyE
  (params (Key :type Key%20Structure :default "None") (ActionValue :type Input%20Action%20Value%20Structure))
  (:Pressed
    (CallFunction|SaveAttributes)))

(event Input|KeyboardEvents|DebugKey1
  (params (Key :type Key%20Structure :default "None") (ActionValue :type Input%20Action%20Value%20Structure))
  (:Pressed
    (Stats|Functions|ModifyStat "NewEnumerator0" "NewEnumerator2" "NewEnumerator9" 5e+01)
    (Development|PrintString "Add Stat")))

(fn GetStatRef
  (params (Stat :type E_Stats_List%20Enum :default "NewEnumerator8"))
  (for (_array_element _array_index) (.AttributeList (Utilities|Struct|BreakF_PlayerAttributes (Variables|Default|GetAttributes)))
    (for (_array_element_2 _array_index_2) (Utilities|Struct|BreakF_SingleAttribute _array_element)
      (if (Utilities|Enum|Equal(Enum) (Utilities|Struct|BreakF_SingleStat _array_element_2) Stat)
        (return _array_element _array_index _array_element_2 _array_index_2)))))

(fn GetStatValue
  (params (Type :type E_StatType%20Enum :default "NewEnumerator3") (Stat :type E_Stats_List%20Enum :default "NewEnumerator8"))
  (bind _stat_return (Stats|Getters|GetStatRef Stat))
  (bind (_default _bonus _total) (Utilities|Struct|BreakF_SingleStat _stat_return))
  (return (Utilities|Select :Index Type :NewEnumerator3 0.0 :NewEnumerator0 _default :NewEnumerator1 _bonus :NewEnumerator2 _total)))

(fn GetAttributeRef
  (params (Attribute :type E_Attribute_List%20Enum :default "NewEnumerator3"))
  (for (_array_element _array_index) (.AttributeList (Utilities|Struct|BreakF_PlayerAttributes (Variables|Default|GetAttributes)))
    (if (Utilities|Enum|Equal(Enum) Attribute (Utilities|Struct|BreakF_SingleAttribute _array_element))
      (return _array_element _array_index))))

(fn GetAttributeValue
  (params (Type :type E_StatType%20Enum :default "NewEnumerator0") (Attribute :type E_Attribute_List%20Enum :default "NewEnumerator3"))
  (bind _return_value (Attributes|Getters|GetAttributeRef Attribute))
  (bind (_default _bonus _total) (Utilities|Struct|BreakF_SingleAttribute _return_value))
  (return (Utilities|Select :Index Type :NewEnumerator3 0.0 :NewEnumerator0 _default :NewEnumerator1 _bonus :NewEnumerator2 _total)))

(fn ModifyAttribute
  (params (Operation :type E_Operations%20Enum :default "NewEnumerator0") (Type :type E_StatType%20Enum :default "NewEnumerator0") (Attribute :type E_Attribute_List%20Enum :default "NewEnumerator3") (Value :type Float%20%28double-precision%29))
  (bind _return_value (Attributes|Getters|GetAttributeValue Type Attribute))
  (bind _returnvalue (+ _return_value Value))
  (bind _returnvalue_2 (- _return_value Value))
  (bind _returnvalue_3 (Utilities|Select :Index Operation :NewEnumerator0 _returnvalue :NewEnumerator1 _returnvalue_2 :NewEnumerator2 Value))
  (switch Utilities|FlowControl|Switch|SwitchonE_StatType Type
    (:NewEnumerator3
      (Development|PrintString "Warning: Modify Attribute - 
Error Stat is set to \"None\"")
      (return))
    (:NewEnumerator0
      _)
    (:NewEnumerator1
      _)
    (:NewEnumerator2
      (Attributes|Function|OperateTotalAttribute Operation Attribute Value)
      (return)))
  (LocalVariables|SetAtt%20Float _return_value)
  (LocalVariables|SetCalc%20Float _returnvalue_3)
  (Attributes|Setters|SetAttribute Type Attribute (Math|Float|Clamp(Float) _returnvalue_3 0.0 99999.0))
  (Attributes|Function|ScalingStats Type Operation (.Return%20Value (Attributes|Getters|GetAttributeRef Attribute)) (Math|Float|SelectFloat Value (LocalVariables|GetAtt%20Float) (> (LocalVariables|GetCalc%20Float) 0.0)))
  (if (and (== Attribute 0) (== Operation 0))
    (Attributes|Function|LevelUp Value))
  (Default|CallUpdateUI)
  (return))

(fn OperateTotalAttribute
  (params (Operation :type E_Operations%20Enum :default "NewEnumerator0") (Attribute :type E_Attribute_List%20Enum :default "NewEnumerator3") (Value :type Float%20%28double-precision%29))
  (switch Utilities|FlowControl|Switch|SwitchonE_Operations Operation
    (:NewEnumerator0
      (Attributes|Function|ModifyAttribute "NewEnumerator0" "NewEnumerator0" Attribute Value))
    (:NewEnumerator1
      (if (>= (- (Attributes|Getters|GetAttributeValue "NewEnumerator1" Attribute) Value) 0.0)
        (Attributes|Function|ModifyAttribute "NewEnumerator1" "NewEnumerator1" Attribute Value)
        (else
          (bind _output_get (LocalVariables|SetStored%20Value (Attributes|Getters|GetAttributeValue "NewEnumerator1" Attribute)))
          (Attributes|Function|ModifyAttribute "NewEnumerator1" "NewEnumerator1" Attribute _output_get)
          (Attributes|Function|ModifyAttribute "NewEnumerator1" "NewEnumerator0" Attribute (- Value (LocalVariables|GetStored%20Value))))))
    (:NewEnumerator2
      (Development|PrintString "Warning: Operate Total Stat 
Unable to Set \"Total\" Value"))))

(fn SetAttribute
  (params (Type :type E_StatType%20Enum :default "NewEnumerator0") (Attribute :type E_Attribute_List%20Enum :default "NewEnumerator3") (Value :type Float%20%28double-precision%29))
  (bind (_return_value _return_index) (Attributes|Getters|GetAttributeRef Attribute))
  (LocalVariables|SetLocal%20Attribute _return_value)
  (LocalVariables|SetLocal%20Index _return_index)
  (switch Utilities|FlowControl|Switch|SwitchonE_StatType Type
    (:NewEnumerator0
      (Utilities|Struct|SetmembersinF_SingleAttribute (LocalVariables|GetLocal%20Attribute) Value (+ Value (Utilities|Struct|BreakF_SingleAttribute (LocalVariables|GetLocal%20Attribute)))))
    (:NewEnumerator1
      (Utilities|Struct|SetmembersinF_SingleAttribute (LocalVariables|GetLocal%20Attribute) Value (+ Value (Utilities|Struct|BreakF_SingleAttribute (LocalVariables|GetLocal%20Attribute)))))
    (:NewEnumerator2
      (Development|PrintString "Set Attribute Error: Can not use Total Enum")
      (return)))
  (Utilities|Array|SetArrayElem (.AttributeList (Utilities|Struct|BreakF_PlayerAttributes (Variables|Default|GetAttributes))) (LocalVariables|GetLocal%20Index) (LocalVariables|GetLocal%20Attribute))
  (return))

(fn ModifyStat
  (params (Operation :type E_Operations%20Enum :default "NewEnumerator0") (Type :type E_StatType%20Enum :default "NewEnumerator0") (Stat :type E_Stats_List%20Enum :default "NewEnumerator8") (Value :type Float%20%28double-precision%29))
  (bind _return_value (Stats|Getters|GetStatValue Type Stat))
  (switch Utilities|FlowControl|Switch|SwitchonE_StatType Type
    (:NewEnumerator3
      (Development|PrintString "Warning: Modify Stat - 
Error Stat is set to \"None\"")
      (return))
    (:NewEnumerator0
      _)
    (:NewEnumerator1
      _)
    (:NewEnumerator2
      (Stats|Functions|OperateTotalStat Operation Stat Value)
      (return)))
  (Stats|Setters|SetStat Type Stat (Math|Float|Clamp(Float) (Utilities|Select :Index Operation :NewEnumerator0 (+ _return_value Value) :NewEnumerator1 (- _return_value Value) :NewEnumerator2 Value) 0.0 99999.0))
  (Stats|Functions|ConditionalStats Stat)
  (Default|CallUpdateUI)
  (return))

(fn SetStat
  (params (Type :type E_StatType%20Enum :default "NewEnumerator0") (Stat :type E_Stats_List%20Enum :default "NewEnumerator8") (Value :type Float%20%28double-precision%29))
  (bind (_attributereturn _attribute_index _stat_return _stat_index) (Stats|Getters|GetStatRef Stat))
  (LocalVariables|SetLocalStat (.Stat%20Return (Stats|Getters|GetStatRef Stat)))
  (switch Utilities|FlowControl|Switch|SwitchonE_StatType Type
    (:NewEnumerator0
      (Utilities|Struct|SetmembersinF_SingleStat (LocalVariables|GetLocalStat) Value (+ Value (Utilities|Struct|BreakF_SingleStat (LocalVariables|GetLocalStat)))))
    (:NewEnumerator1
      (Utilities|Struct|SetmembersinF_SingleStat (LocalVariables|GetLocalStat) Value (+ Value (Utilities|Struct|BreakF_SingleStat (LocalVariables|GetLocalStat)))))
    (:NewEnumerator2
      (Development|PrintString "Unable to Set \"Total\" Stat")
      (return)))
  (Stats|Setters|SetStatMember _attributereturn _attribute_index (LocalVariables|GetLocalStat) _stat_index)
  (return))

(fn SetStatMember
  (params (Attribute :type F%20Single%20Attribute%20Structure%20%28by%20ref%29) (Attribute%20Index :type Integer) (Stat :type F%20Single%20Stat%20Structure%20%28by%20ref%29) (Stat%20Index :type Integer))
  (bind _attributes (Variables|Default|GetAttributes))
  (bind _attributelist (Utilities|Struct|BreakF_PlayerAttributes _attributes))
  (bind _output_get (LocalVariables|SetStat%20Array (.StatsInherit (Utilities|Struct|BreakF_SingleAttribute Attribute))))
  (Utilities|Array|SetArrayElem _output_get Stat%20Index Stat)
  (bind _structout (Utilities|Struct|SetmembersinF_SingleAttribute (Utilities|Array|Get(acopy) _attributelist Attribute%20Index) (LocalVariables|GetStat%20Array)))
  (Utilities|Array|SetArrayElem _attributelist Attribute%20Index _structout)
  (return))

(fn ScalingStats
  (params (Type :type E_StatType%20Enum :default "NewEnumerator0") (Operation :type E_Operations%20Enum :default "NewEnumerator0") (Attribute :type F%20Single%20Attribute%20Structure) (Value :type Float%20%28double-precision%29))
  (for _array_element (Utilities|Struct|BreakF_SingleAttribute Attribute)
    (LocalVariables|SetStat (.Name (Utilities|Struct|BreakF_SingleStat _array_element)))
    (Stats|Setters|SetStat Type (LocalVariables|GetStat) (Math|Float|Clamp(Float) (Utilities|Select :Index Operation :NewEnumerator0 (+ (Utilities|Select :Index Type :NewEnumerator3 0.0 :NewEnumerator0 (.Default (Utilities|Struct|BreakF_SingleStat _array_element)) :NewEnumerator1 (.Bonus (Utilities|Struct|BreakF_SingleStat _array_element)) :NewEnumerator2 0.0) (* (.Scale (Utilities|Struct|BreakF_SingleStat _array_element)) Value)) :NewEnumerator1 (- (Utilities|Select :Index Type :NewEnumerator3 0.0 :NewEnumerator0 (.Default (Utilities|Struct|BreakF_SingleStat _array_element)) :NewEnumerator1 (.Bonus (Utilities|Struct|BreakF_SingleStat _array_element)) :NewEnumerator2 0.0) (* (.Scale (Utilities|Struct|BreakF_SingleStat _array_element)) Value)) :NewEnumerator2 (* (.Scale (Utilities|Struct|BreakF_SingleStat _array_element)) Value)) 0.0 99999.0))
    (Stats|Functions|ConditionalStats (LocalVariables|GetStat))))

(fn ConditionalStats
  (params (Stat :type E_Stats_List%20Enum :default "NewEnumerator8"))
  (switch Utilities|FlowControl|Switch|SwitchonE_Stats_List Stat
    (:NewEnumerator9
      (CallFunction|CheckExp))
    (:NewEnumerator2
      (CallFunction|CheckHealth))
    (:NewEnumerator6
      (CallFunction|CheckMana))))

(fn OperateTotalStat
  (params (Operation :type E_Operations%20Enum :default "NewEnumerator0") (Stat :type E_Stats_List%20Enum :default "NewEnumerator8") (Value :type Float%20%28double-precision%29))
  (switch Utilities|FlowControl|Switch|SwitchonE_Operations Operation
    (:NewEnumerator0
      (Stats|Functions|ModifyStat Operation "NewEnumerator0" Stat Value))
    (:NewEnumerator1
      (if (>= (- (Stats|Getters|GetStatValue "NewEnumerator1" Stat) Value) 0.0)
        (Stats|Functions|ModifyStat "NewEnumerator1" "NewEnumerator0" Stat Value)
        (else
          (bind _output_get (LocalVariables|SetStored%20Value (Stats|Getters|GetStatValue "NewEnumerator1" Stat)))
          (Stats|Functions|ModifyStat "NewEnumerator1" "NewEnumerator1" Stat _output_get)
          (Stats|Functions|ModifyStat "NewEnumerator1" "NewEnumerator0" Stat (- Value (LocalVariables|GetStored%20Value))))))
    (:NewEnumerator2
      (Development|PrintString "Warning: Operate Total Stat 
Unable to Set \"Total\" Value"))))

(fn LevelUp
  (params (Value :type Float%20%28double-precision%29))
  (Attributes|Function|ModifyAttribute "NewEnumerator0" "NewEnumerator0" "NewEnumerator6" (* Value 3.0))
  (Default|CallOnLevelUp))

(fn UseAttributePoint
  (params (Attribute :type E_Attribute_List%20Enum :default "NewEnumerator3"))
  (Attributes|Function|ModifyAttribute "NewEnumerator0" "NewEnumerator0" Attribute 1.0)
  (Attributes|Function|ModifyAttribute "NewEnumerator1" "NewEnumerator0" "NewEnumerator6" 1.0))